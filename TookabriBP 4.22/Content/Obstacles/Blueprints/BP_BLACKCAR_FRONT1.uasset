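; BP_BLACKCAR_FRONT1 is a moving car obstacle for a runner game that either kills the player or gets jumped.
; Tick moves the actor along negative world X at a constant speed, scaled by delta time and without sweeping.
; When its box collision overlaps BP_RunnerCharacter, the character's CHTap flag selects the result: KabriJump with a debug print if set, otherwise DeathWithDelay.
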(event `self.BoxCollision.OnComponentBeginOverlap`
  (params (OverlappedComponent :type "PrimitiveComponent Object Reference") (OtherActor :type "Actor Object Reference") (OtherComp :type "PrimitiveComponent Object Reference") (OtherBodyIndex :type Integer) (bFromSweep :type Boolean) (SweepResult :type "HitResult Structure (by ref)"))
  (bind _asbp_runner_character (cast `/Game/Character/BP_RunnerCharacter` OtherActor))
  (if (`/Game/Character/BP_RunnerCharacter.CH_Tap` _asbp_runner_character)
    (`KismetSystemLibrary.PrintString` "IKABRI")
    (`/Game/Character/BP_RunnerCharacter.KabriJump` _asbp_runner_character)
    (else
      (`/Game/Character/BP_RunnerCharacter.DeathWithDelay` _asbp_runner_character))))

(event `self.ReceiveTick`
  (params (DeltaSeconds :type "Float (single-precision)"))
  (`self.K2_AddActorWorldTransform` (`KismetMathLibrary.Conv_VectorToTransform` (* (`KismetMathLibrary.MakeVector` -900.0) DeltaSeconds))))

(fn `UserConstructionScript`)