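; BP_TRUCK_FRONT is a truck obstacle that moves along negative X at constant speed and kills the runner on contact.
; Its lights start off, and overlapping BoxLightsHorn plays a timeline that drives the intensity of four lights for a flashing warning.
; Overlapping BoxCollision calls DeathWithDelay on BP_RunnerCharacter.
; Tick moves the truck without sweep, and the horn sound call is disconnected, so it never plays.
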(event `self.ReceiveBeginPlay`
  ;[1 1 1] ON BEGIN PLAY LIGHTS OFF
  (`LightComponent.SetIntensity` (`self.LeftPointLight_Left`) 0.0)
  (`LightComponent.SetIntensity` (`self.f`) 0.0)
  (`LightComponent.SetIntensity` (`self.RightPointLight_Left`) 0.0)
  (`LightComponent.SetIntensity` (`self.RightPointLight_Right`) 0.0))

(event `self.BoxLightsHorn.OnComponentBeginOverlap`
  (params (OverlappedComponent :type "PrimitiveComponent Object Reference") (OtherActor :type "Actor Object Reference") (OtherComp :type "PrimitiveComponent Object Reference") (OtherBodyIndex :type Integer) (bFromSweep :type Boolean) (SweepResult :type "HitResult Structure (by ref)"))
  ;[1 1 1] FLASHING LIGHTS + HORN
  (cast `/Game/Character/BP_RunnerCharacter` OtherActor)
  (bind (_direction _newtrack_0) (`Timeline|Timeline_0`)
    (:`Update`
      (`LightComponent.SetIntensity` (`self.LeftPointLight_Left`) (`KismetMathLibrary.Lerp` 0.0 35000.0 _newtrack_0))
      (`LightComponent.SetIntensity` (`self.f`) (`KismetMathLibrary.Lerp` 0.0 35000.0 _newtrack_0))
      (`LightComponent.SetIntensity` (`self.RightPointLight_Left`) (`KismetMathLibrary.Lerp` 0.0 35000.0 _newtrack_0))
      (`LightComponent.SetIntensity` (`self.RightPointLight_Right`) (`KismetMathLibrary.Lerp` 0.0 35000.0 _newtrack_0)))))

(event `self.BoxCollision.OnComponentBeginOverlap`
  (params (OverlappedComponent :type "PrimitiveComponent Object Reference") (OtherActor :type "Actor Object Reference") (OtherComp :type "PrimitiveComponent Object Reference") (OtherBodyIndex :type Integer) (bFromSweep :type Boolean) (SweepResult :type "HitResult Structure (by ref)"))
  ;[1 1 1] EVENT KABRI JUMP OR DEATH
  (bind _asbp_runner_character (cast `/Game/Character/BP_RunnerCharacter` OtherActor))
  (`/Game/Character/BP_RunnerCharacter.DeathWithDelay` _asbp_runner_character))

(event `self.ReceiveTick`
  (params (DeltaSeconds :type "Float (single-precision)"))
  ;[1 1 1] OBSTACLE MOVEMENT
  (`self.K2_AddActorWorldTransform` (`KismetMathLibrary.Conv_VectorToTransform` (* (`KismetMathLibrary.MakeVector` -700.0) DeltaSeconds))))

(fn `UserConstructionScript`)