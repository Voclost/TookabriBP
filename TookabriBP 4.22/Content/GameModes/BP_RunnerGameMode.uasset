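; Game mode for an endless-runner style game that builds the road from segment actors and tracks coins and score.
; BeginPlay lays an opening sequence, each segment spawning at the previous one's GetSpawnPoint transform.
; Once enough static-obstacle roads accumulate, SpawnRoadCD randomly inserts a moving-obstacle Road D after empty padding.
; Past a total-segment cap, A, B and C/D spawners fall back to simple roads to bypass engine world limits.
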(event `self.ReceiveBeginPlay`
  (`self.SpawnRoads`))

(event `SpawnRoads`
  (`self.SpawnStartingRoad`)
  (`self.SpawnSimpleRoad`)
  (for _ (range 2)
    (`self.SpawnRoad_A`)
    (`self.SpawnRoad_B`)
    (`self.SpawnRoad_C/D`)))

(fn `GainCoin`
  ;[1 1 1] Coins +1
  (set `self.Coins` (+ (`self.Coins`) 1))
  ;[1 1 1] Adds 10 points to score after a coin is picked up
  (set `self.Score` (+ (`self.Score`) 10)))

(fn `SpawnEmptyRoad`
  (bind _returnvalue (`|SpawnActorFromClass` "/Game/Roads/Road_Empty.Road_Empty_C" (`self.NextRoadSpawnPoint`) "Undefined" "OverrideRootScale" null null))
  ;[1 1 1] Set Next Road's Spawn Point
  (bind _spawnpoint (`/Game/Roads/Road_Empty.GetSpawnPoint` _returnvalue))
  (set `self.NextRoadSpawnPoint` _spawnpoint)
  ;[1 1 1] Road Spawn Count
  (set `self.TotalRoadsSpawned` (+ (`self.TotalRoadsSpawned`) 1)))

(fn `SpawnRoad_A`
  ;[1 1 1] This is required to bypass engines world limitations
  (if (>= (`self.TotalRoadsSpawned`) 555)
    (for _ (range 2)
      (`self.SpawnSimpleRoad`))
    (else
      (bind _returnvalue (`|SpawnActorFromClass` "/Game/Roads/Road_A.Road_A_C" (`self.NextRoadSpawnPoint`) "Undefined" "OverrideRootScale" null null))
      ;[1 1 1] Set Next Road's Spawn Point
      (bind _spawnpoint (`/Game/Roads/Road_A.GetSpawnPoint` _returnvalue))
      (set `self.NextRoadSpawnPoint` _spawnpoint)
      ;[1 1 1] Road Spawn Count
      (set `self.TotalRoadsSpawned` (+ (`self.TotalRoadsSpawned`) 1))
      ;[1 1 1] Roads with static obstacles
      (set `self.StaticRoads` (+ (`self.StaticRoads`) 1)))))

(fn `SpawnRoad_B`
  ;[1 1 1] This is required to bypass engines world limitations
  (if (>= (`self.TotalRoadsSpawned`) 555)
    (for _ (range 2)
      (`self.SpawnSimpleRoad`))
    (else
      (bind _returnvalue (`|SpawnActorFromClass` "/Game/Roads/Road_B.Road_B_C" (`self.NextRoadSpawnPoint`) "Undefined" "OverrideRootScale" null null))
      ;[1 1 1] Set Next Road's Spawn Point
      (bind _spawnpoint (`/Game/Roads/Road_B.GetSpawnPoint` _returnvalue))
      (set `self.NextRoadSpawnPoint` _spawnpoint)
      ;[1 1 1] Road Spawn Count
      (set `self.TotalRoadsSpawned` (+ (`self.TotalRoadsSpawned`) 1))
      ;[1 1 1] Roads with static obstacles
      (set `self.StaticRoads` (+ (`self.StaticRoads`) 1)))))

(fn `SpawnRoad_C/D`
  ;[1 1 1] This is required to bypass engines world limitations
  (if (>= (`self.TotalRoadsSpawned`) 555)
    (for _ (range 2)
      (`self.SpawnSimpleRoad`))
    (elif (> (`self.StaticRoads`) 15)
      (if (`KismetMathLibrary.RandomBool`)
        ;[1 1 1] Spawn road(Road D) with moving obstacles
        (`self.SpawnEmptyRoad`)
        (`self.SpawnEmptyRoad`)
        (`self.SpawnRoad_D`)
        (bind _returnvalue (`|SpawnActorFromClass` "/Game/Roads/Road_C.Road_C_C" (`self.NextRoadSpawnPoint`) "Undefined" "OverrideRootScale" null null))
        ;[1 1 1] Set Next Road's Spawn Point
        (bind _spawnpoint (`/Game/Roads/Road_C.GetSpawnPoint` _returnvalue))
        (set `self.NextRoadSpawnPoint` _spawnpoint)
        ;[1 1 1] Road Spawn Count
        (set `self.TotalRoadsSpawned` (+ (`self.TotalRoadsSpawned`) 4))
        ;[1 1 1] Reset static road count
        (set `self.StaticRoads` 0)
        (else
          (set `self.StaticRoads` 0)
          (bind _returnvalue_2 (`|SpawnActorFromClass` "/Game/Roads/Road_C.Road_C_C" (`self.NextRoadSpawnPoint`) "Undefined" "OverrideRootScale" null null :!label _label))
          ;[1 1 1] Set Next Road's Spawn Point
          (bind _spawnpoint_2 (`/Game/Roads/Road_C.GetSpawnPoint` _returnvalue_2))
          (set `self.NextRoadSpawnPoint` _spawnpoint_2)
          ;[1 1 1] Road Spawn Count
          (set `self.TotalRoadsSpawned` (+ (`self.TotalRoadsSpawned`) 1))
          ;[1 1 1] Roads with static obstacles
          (set `self.StaticRoads` (+ (`self.StaticRoads`) 1))))
      (else
        (goto _label)))))

(fn `SpawnRoad_CURVE_RIGHT`
  ;[1 1 1] This is required to bypass engines world limitations
  (if (not (>= (`self.TotalRoadsSpawned`) 555))
    (bind _returnvalue (`|SpawnActorFromClass` "/Game/Roads/Road_CURVE_RIGHT.Road_CURVE_RIGHT_C" (`self.NextRoadSpawnPoint`) "Undefined" "OverrideRootScale" null null))
    ;[1 1 1] Set Next Road's Spawn Point
    (bind _spawnpoint (`/Game/Roads/Road_CURVE_RIGHT.GetSpawnPoint` _returnvalue))
    (set `self.NextRoadSpawnPoint` _spawnpoint)
    ;[1 1 1] Road Spawn Count
    (set `self.TotalRoadsSpawned` (+ (`self.TotalRoadsSpawned`) 1))
    ;[1 1 1] Roads with static obstacles
    (set `self.StaticRoads` (+ (`self.StaticRoads`) 1))))

(fn `SpawnRoad_D`
  (bind _returnvalue (`|SpawnActorFromClass` "/Game/Roads/Road_D.Road_D_C" (`self.NextRoadSpawnPoint`) "Undefined" "OverrideRootScale" null null))
  ;[1 1 1] Set Next Road's Spawn Point
  (bind _spawnpoint (`/Game/Roads/Road_D.GetSpawnPoint` _returnvalue))
  (set `self.NextRoadSpawnPoint` _spawnpoint)
  ;[1 1 1] Road Spawn Count
  (set `self.TotalRoadsSpawned` (+ (`self.TotalRoadsSpawned`) 1)))

(fn `SpawnSimpleRoad`
  (bind _returnvalue (`|SpawnActorFromClass` "/Game/Roads/Road_Simple.Road_Simple_C" (`self.NextRoadSpawnPoint`) "Undefined" "OverrideRootScale" null null))
  ;[1 1 1] Set Next Road's Spawn Point
  (bind _spawnpoint (`/Game/Roads/Road_Simple.GetSpawnPoint` _returnvalue))
  (set `self.NextRoadSpawnPoint` _spawnpoint)
  ;[1 1 1] Road Spawn Count
  (set `self.TotalRoadsSpawned` (+ (`self.TotalRoadsSpawned`) 1)))

(fn `SpawnStartingRoad`
  (bind _returnvalue (`|SpawnActorFromClass` "/Game/Roads/Road_Simple.Road_Simple_C" (`self.StartingTransform`) "Undefined" "OverrideRootScale" null null))
  ;[1 1 1] Set Next Road's Spawn Point
  (bind _spawnpoint (`/Game/Roads/Road_Simple.GetSpawnPoint` _returnvalue))
  (set `self.NextRoadSpawnPoint` _spawnpoint)
  ;[1 1 1] Reset Total Roads Spawned
  (set `self.TotalRoadsSpawned` 0))

(fn `UserConstructionScript`)