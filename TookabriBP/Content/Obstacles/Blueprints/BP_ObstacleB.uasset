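; BP_ObstacleB is an obstacle for a runner game that kills the player on contact.
; Overlapping its Box calls Death on BP_RunnerCharacter, ignoring other actors.
; The construction script has a 50% chance to add a coin spawner child actor at the Arrow's relative transform, with a second coin flip choosing between two spawner branches.
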(event `self.Box.OnComponentBeginOverlap`
  (params (OverlappedComponent :type "PrimitiveComponent Object Reference") (OtherActor :type "Actor Object Reference") (OtherComp :type "PrimitiveComponent Object Reference") (OtherBodyIndex :type Integer) (bFromSweep :type Boolean) (SweepResult :type "HitResult Structure (by ref)"))
  (bind _asbp_runner_character (cast `/Game/Character/BP_RunnerCharacter` OtherActor))
  (`/Game/Character/BP_RunnerCharacter.Death` _asbp_runner_character))

(fn `UserConstructionScript`
  ;[1 1 1] 50% chance to spawn one of the coin spawn bps
  (if (`KismetMathLibrary.RandomBool`)
    (if (`KismetMathLibrary.RandomBool`)
      (`AddComponent|NODE_AddChildActorComponent-2` :`RelativeTransform` (`SceneComponent.GetRelativeTransform` (`self.Arrow`)))
      (else
        (`AddComponent|NODE_AddChildActorComponent-1` :`RelativeTransform` (`SceneComponent.GetRelativeTransform` (`self.Arrow`)))))))