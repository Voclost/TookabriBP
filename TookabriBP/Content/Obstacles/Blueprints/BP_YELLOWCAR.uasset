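; BP_YELLOWCAR is a moving car obstacle for the runner character.
; Tick pushes it along negative X at a constant, frame-rate-independent speed without sweeping.
; When its box collision overlaps BP_RunnerCharacter, the character's CHTap flag decides between calling KabriJump and calling Death.
; A separate HornCollision overlap with the runner plays a car horn accident sound at the car's location.
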(event `self.ReceiveBeginPlay`)

(event `self.BoxCollision.OnComponentBeginOverlap`
  (params (OverlappedComponent :type "PrimitiveComponent Object Reference") (OtherActor :type "Actor Object Reference") (OtherComp :type "PrimitiveComponent Object Reference") (OtherBodyIndex :type Integer) (bFromSweep :type Boolean) (SweepResult :type "HitResult Structure (by ref)"))
  ;[1 1 1] EVENT KABRI OR NOT
  (bind _asbp_runner_character (cast `/Game/Character/BP_RunnerCharacter` OtherActor))
  (if (`/Game/Character/BP_RunnerCharacter.CH_Tap` _asbp_runner_character)
    (`/Game/Character/BP_RunnerCharacter.KabriJump` _asbp_runner_character)
    (else
      (`/Game/Character/BP_RunnerCharacter.Death` _asbp_runner_character))))

(event `self.ReceiveTick`
  (params (DeltaSeconds :type "Float (single-precision)"))
  ;[1 1 1] CAR MOVEMENT
  (`self.K2_AddActorWorldTransform` (`KismetMathLibrary.Conv_VectorToTransform` (* (`KismetMathLibrary.MakeVector` -900.0) DeltaSeconds))))

(event `self.HornCollision.OnComponentBeginOverlap`
  (params (OverlappedComponent :type "PrimitiveComponent Object Reference") (OtherActor :type "Actor Object Reference") (OtherComp :type "PrimitiveComponent Object Reference") (OtherBodyIndex :type Integer) (bFromSweep :type Boolean) (SweepResult :type "HitResult Structure (by ref)"))
  ;[1 1 1] HORNCOLLISION BETWEEN CAR AND CHARACTER TO PLAY HORN ACCIDENT
  (cast `/Game/Character/BP_RunnerCharacter` OtherActor)
  (`GameplayStatics.PlaySoundAtLocation` "/Game/Sounds/Cars/car_klaxons_accident_min.car_klaxons_accident_min" (`self.K2_GetActorLocation`)))

(fn `UserConstructionScript`)