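; BP_BACK_CAR_BUS is a runner obstacle combining a bus and a red car that moves along X at constant speed each Tick.
; Overlap boxes report hits to BP_RunnerCharacter: the bus box triggers BusTruckDeath and the left box HitBackBusLeft.
; The red car box triggers KabriJump when the character's CHTap flag is set, otherwise Death.
; The roof-acceleration logic is disconnected, so the bus mesh overlap does nothing.
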(event `self.BUS_MESH.OnComponentBeginOverlap`
  (params (OverlappedComponent :type "PrimitiveComponent Object Reference") (OtherActor :type "Actor Object Reference") (OtherComp :type "PrimitiveComponent Object Reference") (OtherBodyIndex :type Integer) (bFromSweep :type Boolean) (SweepResult :type "HitResult Structure (by ref)"))
  ;[1 1 1] ROOF ACCELERATE
)

(event `self.BoxCollision.OnComponentBeginOverlap`
  (params (OverlappedComponent :type "PrimitiveComponent Object Reference") (OtherActor :type "Actor Object Reference") (OtherComp :type "PrimitiveComponent Object Reference") (OtherBodyIndex :type Integer) (bFromSweep :type Boolean) (SweepResult :type "HitResult Structure (by ref)"))
  ;[1 1 1] EVENT KABRI JUMP OR DEATH
  (bind _asbp_runner_character (cast `/Game/Character/BP_RunnerCharacter` OtherActor))
  (`/Game/Character/BP_RunnerCharacter.BusTruckDeath` _asbp_runner_character))

(event `self.BoxHitLeft.OnComponentBeginOverlap`
  (params (OverlappedComponent :type "PrimitiveComponent Object Reference") (OtherActor :type "Actor Object Reference") (OtherComp :type "PrimitiveComponent Object Reference") (OtherBodyIndex :type Integer) (bFromSweep :type Boolean) (SweepResult :type "HitResult Structure (by ref)"))
  (bind _asbp_runner_character (cast `/Game/Character/BP_RunnerCharacter` OtherActor))
  (`/Game/Character/BP_RunnerCharacter.HitBackBusLeft` _asbp_runner_character))

(event `self.ReceiveTick`
  (params (DeltaSeconds :type "Float (single-precision)"))
  ;[1 1 1] OBSTACLE MOVEMENT
  (`self.K2_AddActorWorldTransform` (`KismetMathLibrary.Conv_VectorToTransform` (* (`KismetMathLibrary.MakeVector` 400.0) DeltaSeconds))))

(event `self.RED_CAR_BOX.OnComponentBeginOverlap`
  (params (OverlappedComponent :type "PrimitiveComponent Object Reference") (OtherActor :type "Actor Object Reference") (OtherComp :type "PrimitiveComponent Object Reference") (OtherBodyIndex :type Integer) (bFromSweep :type Boolean) (SweepResult :type "HitResult Structure (by ref)"))
  ;[1 1 1] EVENT CAR KABRI OR DEATH
  (bind _asbp_runner_character (cast `/Game/Character/BP_RunnerCharacter` OtherActor))
  (if (`/Game/Character/BP_RunnerCharacter.CH_Tap` _asbp_runner_character)
    (`KismetSystemLibrary.PrintString` "IKABRI")
    (`/Game/Character/BP_RunnerCharacter.KabriJump` _asbp_runner_character)
    (else
      (`/Game/Character/BP_RunnerCharacter.Death` _asbp_runner_character))))

(fn `UserConstructionScript`)